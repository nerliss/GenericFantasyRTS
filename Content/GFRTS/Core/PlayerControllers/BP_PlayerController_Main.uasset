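; Main RTS player controller that defines edge-scroll camera movement from the mouse position.
; BeginPlay locks the mouse to the viewport in Game and UI input mode and caches the view target as the camera.
; Four Move functions offset the camera root, scaling scroll speed by cursor depth into edge bands, which are wider at top and left.
; Tick is empty, so nothing in this graph calls them.
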(event EventBeginPlay
  (Input|SetInputModeGameandUI self 0 "LockAlways" false)
  (Variables|Default|SetRTSCameraRef (Pawn|GetViewTarget)))

(event EventTick
  (params (DeltaSeconds :type Float%20%28single-precision%29)))

(fn ConstructionScript)

(fn MoveDown
  (bind _returnvalue (Viewport|GetViewportSize))
  (bind _returnvalue_2 (Class|WidgetLayoutLibrary|GetMousePositiononViewport))
  (Transformation|AddRelativeLocation (Variables|/Script/Engine.Actor|GetRootComponent (Variables|Default|GetRTSCameraRef)) (* (Math|Float|Clamp(Float) (Math|Float|NormalizetoRange (.y _returnvalue_2) (* (.y _returnvalue) 0.95) (.y _returnvalue))) (Math|Vector|MakeVector 0.0 (* (Variables|Default|GetCameraScrollSpeed) -1.0) 0.0)) false false))

(fn MoveUp
  (bind _returnvalue (Class|WidgetLayoutLibrary|GetMousePositiononViewport))
  (Transformation|AddRelativeLocation (Variables|/Script/Engine.Actor|GetRootComponent (Variables|Default|GetRTSCameraRef)) (* (- 1.0 (Math|Float|Clamp(Float) (Math|Float|NormalizetoRange (.y _returnvalue) 0.0 (* (.y (Viewport|GetViewportSize)) 0.2)))) (Math|Vector|MakeVector 0.0 (Variables|Default|GetCameraScrollSpeed) 0.0)) false false))

(fn MoveRight
  (bind _returnvalue (Viewport|GetViewportSize))
  (bind _returnvalue_2 (Class|WidgetLayoutLibrary|GetMousePositiononViewport))
  (Transformation|AddRelativeLocation (Variables|/Script/Engine.Actor|GetRootComponent (Variables|Default|GetRTSCameraRef)) (* (Math|Float|Clamp(Float) (Math|Float|NormalizetoRange (.x _returnvalue_2) (* (.x _returnvalue) 0.95) (.x _returnvalue))) (Math|Vector|MakeVector (* (Variables|Default|GetCameraScrollSpeed) -1.0) 0.0 0.0)) false false))

(fn MoveLeft
  (bind _returnvalue (Class|WidgetLayoutLibrary|GetMousePositiononViewport))
  (Transformation|AddRelativeLocation (Variables|/Script/Engine.Actor|GetRootComponent (Variables|Default|GetRTSCameraRef)) (* (- 1.0 (Math|Float|Clamp(Float) (Math|Float|NormalizetoRange (.x _returnvalue) 0.0 (* (.x (Viewport|GetViewportSize)) 0.2)))) (Math|Vector|MakeVector (Variables|Default|GetCameraScrollSpeed) 0.0 0.0)) false false))